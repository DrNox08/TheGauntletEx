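; Player controller for the Gauntlet game that owns the pause menu and switches input between gameplay and UI.
; On BeginPlay it creates the pause menu widget, adds it to the viewport collapsed and sets game-only input.
; DoPause shows the menu with focused UI-only input and a mouse cursor, and Unpause reverses this.
; Neither function pauses the game itself, only visibility, input mode and cursor change.
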(event `self.ReceiveBeginPlay`
  (bind _returnvalue (`|CreateWidget` "/Game/Game/Widget/WBP_PauseMenu.WBP_PauseMenu_C" self))
  (bind _output_get (set `self.Pause Menu` _returnvalue))
  (`UserWidget.AddToViewport` _output_get 0)
  (`Widget.SetVisibility` _output_get "Collapsed")
  (`WidgetBlueprintLibrary.SetInputMode_GameOnly` self))

(fn `DoPause`
  (bind _pause_menu (`self.Pause Menu`))
  (`Widget.SetVisibility` _pause_menu "Visible")
  (`WidgetBlueprintLibrary.SetInputMode_UIOnlyEx` self _pause_menu "DoNotLock" true)
  (set `self.bShowMouseCursor` true))

(fn `Unpause`
  (`Widget.SetVisibility` (`self.Pause Menu`) "Collapsed")
  (`WidgetBlueprintLibrary.SetInputMode_GameOnly` self true)
  (set `self.bShowMouseCursor` false))

(fn `UserConstructionScript`)