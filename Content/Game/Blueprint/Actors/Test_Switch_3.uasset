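; Test switch actor that turns green when the MainCharacter enters its collision box and red again when its gate resets switches.
; On overlap it swaps the mesh material, calls TouchTriggered and prints the result for debugging.
; At BeginPlay it binds to the referenced GateActor's OnResetSwitches dispatcher, which drives the change back to red.
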(event `self.ReceiveBeginPlay`
  (add `Gate.OnResetSwitches` (`self.GateActor`) (delegate `CustomEvent`)))

(event `CustomEvent`
  (`PrimitiveComponent.SetMaterial` (`self.SwitchMesh`) 0 "/Game/Game/Materials/M_RedSimple.M_RedSimple"))

(event `self.BoxCollision.OnComponentBeginOverlap`
  (params (OverlappedComponent :type "PrimitiveComponent Object Reference") (OtherActor :type "Actor Object Reference") (OtherComp :type "PrimitiveComponent Object Reference") (OtherBodyIndex :type Integer) (bFromSweep :type Boolean) (SweepResult :type "HitResult Structure (by ref)"))
  (cast `MainCharacter` OtherActor)
  (`PrimitiveComponent.SetMaterial` (`self.SwitchMesh`) 0 "/Game/Game/Materials/M_GreenSimple.M_GreenSimple")
  (bind _returnvalue (`self.TouchTriggered`))
  (`KismetSystemLibrary.PrintString` (`KismetStringLibrary.Conv_IntToString` _returnvalue)))

(fn `UserConstructionScript`)